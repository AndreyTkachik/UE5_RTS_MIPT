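; RTS-style player controller that routes Enhanced Input to camera movement and building placement, and creates the main UI.
; Camera pawn's movement component handles move, zoom, gated mouse panning and edge scroll.
; Tick feeds a cursor line trace to BuildingManager and pushes resources to the UI.
; Primary action in Construction mode spawns validated previews, then returns to Selection; V spawns a unit at the cursor.
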(event `self.ReceiveTick`
  (params (DeltaSeconds :type "Float (single-precision)"))
  (bind _output_get (set `self.MousePosition` (`self.SetMousePosition` (+ (`/Game/Core/Player/BP_CameraPawn.GetCurrentArmLength` (`self.CameraPawnReference`)) 3000.0))))
  (`/Game/Core/Buildings/BP_BuildingManager.SetMousePosition` (`self.BuildingManager`) _output_get)
  (`self.EventSetResources`))

(event `self.ReceiveBeginPlay`
  (`|ExecutionSequence`
    (:`then_0`
      (`EnhancedInputSubsystemInterface.AddMappingContext` (subsystem `EnhancedInputLocalPlayerSubsystem`) "/Game/Core/Player/Inputs/IMC_RTS.IMC_RTS" 0 (struct))
      (set `self.bShowMouseCursor` true)
      (bind _asbp_camera_pawn (cast `/Game/Core/Player/BP_CameraPawn` (`GameplayStatics.GetPlayerPawn` 0)))
      (bind _output_get (set `self.CameraPawnReference` _asbp_camera_pawn))
      (set `self.CameraMovementReference` (`/Game/Core/Player/BP_CameraPawn.PawnMovementController` _output_get)))
    (:`then_1`
      (bind _returnvalue (`|CreateWidget` "/Game/Core/Widgets/WBP_MainUI.WBP_MainUI_C" self))
      (bind _output_get_2 (set `self.MainWidgetRef` _returnvalue))
      (`UserWidget.AddToViewport` _output_get_2 0)
      (`WidgetBlueprintLibrary.SetInputMode_GameAndUIEx` self _output_get_2 "LockInFullscreen" false))))

(event `EnhancedInput|/Game/Core/Player/Inputs/IA_Move`
  (params (ActionValue :type "Vector2D Structure") (ElapsedSeconds :type "Float (double-precision)") (TriggeredSeconds :type "Float (double-precision)") (InputAction :type "InputAction Object Reference" :default "/Game/Core/Player/Inputs/IA_Move.IA_Move"))
  (:`Triggered`
    (`/Game/Core/Player/BP_ActorMovementComp.BasicMovementsControl` (`self.CameraMovementReference`) ActionValue_X ActionValue_Y)))

(event `EnhancedInput|/Game/Core/Player/Inputs/IA_RotatePreview`
  (params (ActionValue :type "Float (double-precision)") (ElapsedSeconds :type "Float (double-precision)") (TriggeredSeconds :type "Float (double-precision)") (InputAction :type "InputAction Object Reference" :default "/Game/Core/Player/Inputs/IA_RotatePreview.IA_RotatePreview"))
  (bind _buildingmanager (`self.BuildingManager`))
  (:`Triggered`
    (switch `int` (`KismetMathLibrary.FTrunc` ActionValue)
      (:`-1`
        (`/Game/Core/Buildings/BP_BuildingManager.RotatePreviewLeft` _buildingmanager))
      (:`1`
        (`/Game/Core/Buildings/BP_BuildingManager.RotatePreviewRight` _buildingmanager)))))

(event `EnhancedInput|/Game/Core/Player/Inputs/IA_ZoomIn`
  (params (ActionValue :type Boolean) (ElapsedSeconds :type "Float (double-precision)") (TriggeredSeconds :type "Float (double-precision)") (InputAction :type "InputAction Object Reference" :default "/Game/Core/Player/Inputs/IA_ZoomIn.IA_ZoomIn"))
  (:`Triggered`
    (`/Game/Core/Player/BP_ActorMovementComp.ZoomIn` (`self.CameraMovementReference`))))

(event `EnhancedInput|/Game/Core/Player/Inputs/IA_ZoomOut`
  (params (ActionValue :type Boolean) (ElapsedSeconds :type "Float (double-precision)") (TriggeredSeconds :type "Float (double-precision)") (InputAction :type "InputAction Object Reference" :default "/Game/Core/Player/Inputs/IA_ZoomOut.IA_ZoomOut"))
  (:`Triggered`
    (`/Game/Core/Player/BP_ActorMovementComp.ZoomOut` (`self.CameraMovementReference`))))

(event `EnhancedInput|/Game/Core/Player/Inputs/IA_ZoomReset`
  (params (ActionValue :type Boolean) (ElapsedSeconds :type "Float (double-precision)") (TriggeredSeconds :type "Float (double-precision)") (InputAction :type "InputAction Object Reference" :default "/Game/Core/Player/Inputs/IA_ZoomReset.IA_ZoomReset"))
  (:`Started`
    (`/Game/Core/Player/BP_ActorMovementComp.ResetZoom` (`self.CameraMovementReference`))))

(event `/Game/Core/Interfaces/BPI_GameTime.SetDate`
  (params (DateTimeStructure :type "DateTime Structure"))
  (message `/Game/Core/Interfaces/BPI_GameTime.SetDate` (`self.MainWidgetRef`) DateTimeStructure))

(event `EventSetResources`
  (message `/Game/Core/Interfaces/BPI_Resources.SetResources` (`self.MainWidgetRef`) (`self.BaseMaterialResource`) (`self.EnergyResource`)))

(event `InputAxisKey|MouseX`
  (params (AxisValue :type "Float (single-precision)"))
  (`/Engine/EditorBlueprintResources/StandardMacros.Gate` true :!label _label
    (:`Exit`
      (`/Game/Core/Player/BP_ActorMovementComp.PanCamera` (`self.CameraMovementReference`) (* AxisValue 5.0)))))

(event `EnhancedInput|/Game/Core/Player/Inputs/IA_Pan`
  (params (ActionValue :type Boolean) (ElapsedSeconds :type "Float (double-precision)") (TriggeredSeconds :type "Float (double-precision)") (InputAction :type "InputAction Object Reference" :default "/Game/Core/Player/Inputs/IA_Pan.IA_Pan"))
  (bind _cameramovementreference (`self.CameraMovementReference`))
  (:`Triggered`
    (`/Game/Core/Player/BP_ActorMovementComp.SetDisableEdgeScroll` _cameramovementreference true)
    (goto _label :!via `Open`))
  (:`Canceled`
    (`/Game/Core/Player/BP_ActorMovementComp.SetDisableEdgeScroll` _cameramovementreference true :!label _label_2)
    (goto _label :!via `Close`))
  (:`Completed`
    (goto _label_2)))

(event `EnhancedInput|/Game/Core/Player/Inputs/IA_PanReset`
  (params (ActionValue :type Boolean) (ElapsedSeconds :type "Float (double-precision)") (TriggeredSeconds :type "Float (double-precision)") (InputAction :type "InputAction Object Reference" :default "/Game/Core/Player/Inputs/IA_PanReset.IA_PanReset"))
  (:`Started`
    (`/Game/Core/Player/BP_ActorMovementComp.ResetPan` (`self.CameraMovementReference`))))

(event `EnhancedInput|/Game/Core/Player/Inputs/IA_ResetCamera`
  (params (ActionValue :type Boolean) (ElapsedSeconds :type "Float (double-precision)") (TriggeredSeconds :type "Float (double-precision)") (InputAction :type "InputAction Object Reference" :default "/Game/Core/Player/Inputs/IA_ResetCamera.IA_ResetCamera"))
  (:`Started`
    (`/Game/Core/Player/BP_ActorMovementComp.ResetCamera` (`self.CameraMovementReference`))))

(event `InputAxisKey|MouseX`
  (params (AxisValue :type "Float (single-precision)"))
  (`/Game/Core/Player/BP_ActorMovementComp.EdgeScroll` (`self.CameraMovementReference`) :!label _label_3))

(event `InputAxisKey|MouseY`
  (params (AxisValue :type "Float (single-precision)"))
  (goto _label_3))

(event `EnhancedInput|/Game/Core/Player/Inputs/IA_PrimaryAction`
  (params (ActionValue :type Boolean) (ElapsedSeconds :type "Float (double-precision)") (TriggeredSeconds :type "Float (double-precision)") (InputAction :type "InputAction Object Reference" :default "/Game/Core/Player/Inputs/IA_PrimaryAction.IA_PrimaryAction"))
  (:`Triggered`
    (switch `/Game/Core/Enums/Player/EPrimaryActionModes` (`self.ActionMode`)
      (:`NewEnumerator1`
        (`self.ConstructionEvents`)))))

(event `/Game/Core/Interfaces/BPI_Construction.StartPreview`
  (params (RowName :type Name))
  (if (`/Game/Core/Buildings/BP_BuildingManager.GetIsPreviewing` (`self.BuildingManager`))
    (`/Game/Core/Buildings/BP_BuildingManager.DestroyPreview` (`self.BuildingManager`)))
  (`/Game/Core/Buildings/BP_BuildingManager.SetPreview` (`self.BuildingManager`) RowName)
  (`self.SetActionMode` "NewEnumerator1"))

(event `Key|V`
  (params (Key :type "Key Structure"))
  (bind (_relativelocationingame_x _relativelocationingame_y) (`KismetMathLibrary.BreakVector` (`/Game/Core/Library/BP_FunctionLibrary.SetCursorWorldPosition` self 10000.0)))
  (:`Pressed`
    (`|SpawnActorFromClass` "/Game/Core/Units/BP_UnitMaster.BP_UnitMaster_C" (`KismetMathLibrary.MakeTransform` (`KismetMathLibrary.MakeVector` _relativelocationingame_x _relativelocationingame_y 200.0)) "AdjustIfPossibleButAlwaysSpawn" "MultiplyWithRoot" null null)))

(fn `ConstructionChecks`
  (returns (ValidBuild :type Boolean))
  (bind _buildingmanager (`self.BuildingManager`))
  (if (`/Game/Core/Buildings/BP_BuildingManager.GetIsPreviewValid` (`self.BuildingManager`))
    (if (and (not (`/Game/Core/Buildings/BP_BuildingManager.GetIsPreviewOverlapping` _buildingmanager)) (not (`/Game/Core/Buildings/BP_BuildingManager.GetIsPreviewOnSlope` _buildingmanager)))
      (if true
        (return true)
        (else
          _))))
  (return false))

(fn `ConstructionEvents`
  (bind _validbuild (`self.ConstructionChecks`))
  (if _validbuild
    (`self.RemovePreview`)
    (`/Game/Core/Buildings/BP_BuildingManager.SpawnConstruction` (`self.BuildingManager`))
    (`self.SetActionMode` "NewEnumerator0")))

(fn `RemovePreview`
  (bind _buildingmanager (`self.BuildingManager`))
  (`/Game/Core/Buildings/BP_BuildingManager.StoreVariables` _buildingmanager)
  (`/Game/Core/Buildings/BP_BuildingManager.DestroyPreview` _buildingmanager))

(fn `SetActionMode`
  (params (ActionMode :type "/Game/Core/Enums/Player/EPrimaryActionModes Enum" :default "NewEnumerator0"))
  (set `self.ActionMode` ActionMode)
  (return))

(fn `SetMousePosition`
  (params (TraceDistance :type "Float (double-precision)"))
  (returns (RelativeCursorLocation :type "Vector Structure"))
  (bind (_worldlocation _worlddirection) (`self.DeprojectMousePositionToWorld`))
  (bind _outhit (`KismetSystemLibrary.LineTraceSingle` _worldlocation (+ _worldlocation (* _worlddirection TraceDistance)) "TraceTypeQuery3"))
  (bind (_bblockinghit _binitialoverlap _time _distance _location _impactpoint _normal _impactnormal _physmat _hitactor) (`GameplayStatics.BreakHitResult` _outhit))
  (if (!= _hitactor null)
    (return _location)))

(fn `UserConstructionScript`)
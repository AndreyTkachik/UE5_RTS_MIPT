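; BP_CameraPawn is a camera pawn that keeps itself at a target height above the surface below.
; BeginPlay initializes its PawnMovementController component.
; Each tick a downward trace measures ground distance, snapping the pawn down when too high and raising it by a fixed step when too low.
; Helper functions set the camera boom's arm length from a zoom curve and return the current length.
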(event `self.ReceiveBeginPlay`
  (`/Game/Core/Player/BP_ActorMovementComp.InitComponent` (`self.PawnMovementController`)))

(event `self.ReceiveTick`
  (params (DeltaSeconds :type "Float (single-precision)"))
  (`self.AdjustCameraHight`))

(fn `AdjustCameraHight`
  (locals (Distance_Local :type "Float (double-precision)" :default 0.0))
  (bind _returnvalue (`self.K2_GetActorLocation`))
  (bind _outhit (`KismetSystemLibrary.LineTraceSingle` _returnvalue (- _returnvalue (0.0 0.0 100000.0)) "TraceTypeQuery3"))
  (set `local.Distance_Local` (`KismetMathLibrary.VSize` (- (`.ImpactPoint` (`GameplayStatics.BreakHitResult` _outhit)) (`self.K2_GetActorLocation`))))
  (if (`KismetMathLibrary.NearlyEqual_FloatFloat` (`local.Distance_Local`) (`self.TargetPawnHeight`) 0.1)
    _
    (elif (> (`local.Distance_Local`) (`self.TargetPawnHeight`))
      (`self.K2_SetActorLocation` (- (`self.K2_GetActorLocation`) (`KismetMathLibrary.MakeVector` 0.0 0.0 (- (`local.Distance_Local`) (`self.TargetPawnHeight`)))))
      (else
        (`self.K2_SetActorLocation` (+ (`self.K2_GetActorLocation`) (0.0 0.0 290.0))))))
  (return))

(fn `GetCurrentArmLength`
  (returns (`Target Arm Length` :type "Float (single-precision)"))
  (return (`SpringArmComponent.TargetArmLength` (`self.CameraBoom`))))

(fn `SetArmLength`
  (params (InZoomAmount :type "Float (double-precision)"))
  (bind _curvezoomarmlngt (`self.CurveZoomArmLngt`)
    (:`then`
      (set `SpringArmComponent.TargetArmLength` (`CurveFloat.GetFloatValue` _curvezoomarmlngt InZoomAmount) (`self.CameraBoom`)))
    (:`else`
      _))
  (return))

(fn `UserConstructionScript`)
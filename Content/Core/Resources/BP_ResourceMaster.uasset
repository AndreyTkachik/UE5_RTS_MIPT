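; BP_ResourceMaster is a resource actor Blueprint, apparently the parent for resources such as Base Materials and Energy.
; Its construction script runs setup only for visible types, as decided by IsResourceVisible from ResourceName: Base Materials is visible, Energy is not.
; Setup derives CurrentResources from StartResources and the Full or Depleted ResourceState, then gives ResourceMesh a random world yaw.
; The event graph holds no runtime logic.
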(fn `IsResourceVisible`
  (returns (Check :type Boolean))
  (switch `/Game/Core/Enums/Resources/EResourcesTypes` (`self.ResourceName`)
    (:`NewEnumerator0`
      (return true))
    (:`NewEnumerator1`
      (return false))))

(fn `UserConstructionScript`
  (if (`self.IsResourceVisible`)
    (switch `/Game/Core/Enums/Resources/EResourcesState` (`self.ResourceState`)
      (:`NewEnumerator0`
        (set `self.ResourceModifier` 0.0))
      (:`NewEnumerator1`
        (set `self.ResourceModifier` 1.0)))
    (set `self.CurrentResources` (* (`self.StartResources`) (`self.ResourceModifier`)))
    (`SceneComponent.K2_SetWorldRotation` (`self.ResourceMesh`) (`KismetMathLibrary.MakeRotator` 0.0 0.0 (`KismetMathLibrary.RandomFloatInRange` 0.0 360.0)) false false)))
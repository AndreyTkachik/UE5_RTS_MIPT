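; BP_SpawnVolume is a volume actor that scatters a resource actor class over landscape within its bounds, optionally on BeginPlay.
; SpawnResource loops by the requested amount, box-tracing on Visibility between random XY points in the actor bounds, offset up and down in Z.
; It spawns the resource at the hit location only when the hit actor is a Landscape, with no retry, so other hits yield no spawn.
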(event `self.ReceiveBeginPlay`
  (if (`self.bIsSpawnedOnBeginPlay`)
    (`self.SpawnResource` (`self.ResourceRef`) (`self.ResourceAmount`))))

(fn `SpawnResource`
  (params (Resource :type "/Game/Core/Resources/BP_ResourceMaster Class Reference") (SpawnAmount :type Integer))
  (locals (ResLocal :type "/Game/Core/Resources/BP_ResourceMaster Class Reference") (SpawnAmountLocal :type Integer))
  (bind (_origin _boxextent) (`self.GetActorBounds` false true))
  (bind _returnvalue (+ (`KismetMathLibrary.MakeVector` (`KismetMathLibrary.RandomFloatInRange` (- 0.0 (.x _boxextent)) (.x _boxextent)) (`KismetMathLibrary.RandomFloatInRange` (- 0.0 (.y _boxextent)) (.y _boxextent)) (.z _origin)) _origin))
  (set `local.ResLocal` Resource)
  (bind _output_get (set `local.SpawnAmountLocal` SpawnAmount))
  (for _ (range (+ _output_get 1))
    (bind _outhit (`KismetSystemLibrary.BoxTraceSingle` (+ _returnvalue (0.0 0.0 270.0)) (- _returnvalue (0.0 0.0 270.0)) (0.0 0.0 0.0) (struct) "TraceTypeQuery1"))
    (bind (_bblockinghit _binitialoverlap _time _distance _location _impactpoint _normal _impactnormal _physmat _hitactor) (`GameplayStatics.BreakHitResult` _outhit))
    (if (== (`GameplayStatics.GetObjectClass` _hitactor) "/Script/Landscape.Landscape")
      (`|SpawnActorFromClass` (`local.ResLocal`) (`KismetMathLibrary.Conv_VectorToTransform` _location) "AdjustIfPossibleButAlwaysSpawn" "MultiplyWithRoot" null null))))

(fn `UserConstructionScript`)
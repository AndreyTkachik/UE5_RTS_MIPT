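; Game state that runs the in-game clock and calendar, starting from its time variables and pausing when GameSpeed is zero.
; Each tick it advances a decimal-hour GameTime through CalculateGameTime, converts it to hours, minutes and seconds, and rolls days, months and years.
; It then sends GameTime to the first BP_SunRotation found at BeginPlay and the DateTime struct to player controller 0 via message calls.
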(event `self.ReceiveBeginPlay`
  (`self.SetInitialGameTime`)
  (`self.GetSunRotActor`))

(event `self.ReceiveTick`
  (params (DeltaSeconds :type "Float (single-precision)"))
  (if (!= (`self.GameSpeed`) 0.0)
    (`self.CalculateTime` DeltaSeconds)
    (`self.SetClockCalendar`)
    (`self.PassGameTime`)
    (`self.PassDateStruct`)))

(event `CalculateTime`
  (params (DeltaTime :type "Float (double-precision)"))
  (bind (_outgametime _gameday) (`/Game/Core/Library/BP_GameTimeLibrary.CalculateGameTime` DeltaTime (`self.GameSpeed`) (`self.GameTime`)))
  (set `self.GameTime` _outgametime)
  (set `self.DayCounter` _gameday))

(event `SetClockCalendar`
  (bind (_year _month _day _hours _minutes _seconds) (`self.UpdateClockCalendar`))
  (`self.SetDateTime` _year _month _day _hours _minutes _seconds))

(event `GetSunRotActor`
  (bind _outactors (`GameplayStatics.GetAllActorsOfClass` "/Game/Core/Actors/BP_SunRotation.BP_SunRotation_C"))
  (for _array_element _outactors
    (set `self.SunActorReference` _array_element)
    (break)))

(event `PassGameTime`
  (bind _sunactorreference (`self.SunActorReference`)
    (:`then`
      (message `/Game/Core/Interfaces/BPI_GameTime.SetGameTime` _sunactorreference (`self.GameTime`)))
    (:`else`)))

(event `PassDateStruct`
  (message `/Game/Core/Interfaces/BPI_GameTime.SetDate` (`GameplayStatics.GetPlayerController` 0) (`self.DateTimeStructure`)))

(fn `SetDateTime`
  (params (Year :type "Integer (by ref)") (Month :type "Integer (by ref)") (Day :type "Integer (by ref)") (Hour :type "Integer (by ref)") (Minute :type "Integer (by ref)") (Second :type "Integer (by ref)"))
  (set `self.DateTimeStructure` (`KismetMathLibrary.MakeDateTime` Year Month Day Hour Minute Second)))

(fn `SetInitialGameTime`
  (set `self.GameTime` (+ (`self.Hours`) (/ (`KismetMathLibrary.Conv_IntToDouble` (`self.Seconds`)) 3600.0) (/ (`KismetMathLibrary.Conv_IntToDouble` (`self.Minutes`)) 60.0))))

(fn `UpdateClockCalendar`
  (returns (Year :type Integer) (Month :type Integer) (Day :type Integer) (Hours :type Integer) (Minutes :type Integer) (Seconds :type Integer))
  (bind (_remainder _returnvalue) (`KismetMathLibrary.FMod` (* (`self.GameTime`) 3600.0) 60.0))
  (bind (_remainder_2 _returnvalue_2) (`KismetMathLibrary.FMod` (`KismetMathLibrary.Conv_IntToDouble` _returnvalue) 60.0))
  (set `self.Seconds` (`KismetMathLibrary.FFloor` _remainder))
  (set `self.Minutes` (`KismetMathLibrary.FFloor` _remainder_2))
  (set `self.Hours` (`KismetMathLibrary.FFloor` (`KismetMathLibrary.FMod` (`KismetMathLibrary.Conv_IntToDouble` _returnvalue_2) 60.0)))
  (bind _output_get (set `self.Day` (+ (`self.Day`) (`self.DayCounter`))))
  (if (> _output_get (`KismetMathLibrary.DaysInMonth` (`self.Year`) (`self.Month`)))
    (set `self.Day` 1)
    (set `self.Month` (+ (`self.Month`) 1)))
  (if (> (`self.Month`) 12)
    (set `self.Month` 1)
    (set `self.Year` (+ (`self.Year`) 1)))
  (return (`self.Year`) (`self.Month`) (`self.Day`) (`self.Hours`) (`self.Minutes`) (`self.Seconds`)))

(fn `UserConstructionScript`)
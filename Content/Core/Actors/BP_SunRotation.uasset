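; BP_SunRotation is an actor that rotates a referenced sun actor to match the game's time of day.
; Each tick it sets the sun's rotation from a pitch that maps GameTime, wrapped to 24 hours, onto a full circle with a 90 degree offset.
; A SetGameTime event updates the stored time, and the actor destroys itself at BeginPlay if no sun reference is valid.
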(event `self.ReceiveBeginPlay`
  (`self.SunReference`
    (:`then`)
    (:`else`
      (`self.K2_DestroyActor`))))

(event `self.ReceiveTick`
  (params (DeltaSeconds :type "Float (single-precision)"))
  (bind _sunreference (`self.SunReference`)
    (:`then`
      (`self.K2_SetActorRotation` _sunreference (`self.CalculateSunRotation`) false))
    (:`else`)))

(event `/Game/Core/Interfaces/BPI_GameTime.SetGameTime`
  (params (GameTime :type "Float (double-precision)"))
  (set `self.GameTime` GameTime))

(fn `CalculateSunRotation`
  (returns (ReturnValue :type "Rotator Structure"))
  (return (`KismetMathLibrary.MakeRotator` 0.0 (+ (* (/ (mod (`self.GameTime`) 24.0) 24.0) 360.0) 90.0))))

(fn `UserConstructionScript`)
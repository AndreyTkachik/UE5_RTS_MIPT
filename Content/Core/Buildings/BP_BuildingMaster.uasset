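; Base building actor that serves as both placement ghost and placed building, tracking construction status and time.
; A DT_Buildings row supplies meshes per status and stage, whose bounds size the collision and entrance boxes.
; Moving the preview runs five slope traces and a box trace that snaps height to the ground.
; Dynamic materials tint the ghost red on overlap or excessive slope, green otherwise.
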(event `self.ReceiveBeginPlay`
  (if (!= (`self.RowName`) "NULL")
    (`|ExecutionSequence`
      (:`then_0`
        (switch `/Game/Core/Enums/Buildings/EConstructuionStatus` (`self.ConstructionStatus`)
          (:`NewEnumerator0`
            (`self.RunSetPreviewMesh`))))
      (:`then_1`
        (switch `/Game/Core/Enums/Buildings/EConstructuionStatus` (`self.ConstructionStatus`)
          (:`NewEnumerator0`
            (`SceneComponent.K2_AttachToComponent` (`self.EntryPoint`) (`self.CurrentBuildingMash`) "None" "KeepRelative" "KeepRelative" "KeepRelative" true)
            (`SceneComponent.K2_AttachToComponent` (`self.CollisionBox`) (`self.CurrentBuildingMash`) "None" "KeepRelative" "KeepRelative" "KeepRelative" true)))))
    (else
      (`self.K2_DestroyActor`))))

(event `SetConstructionStatus`
  (params (ConstructionStatus :type "/Game/Core/Enums/Buildings/EConstructuionStatus Enum" :default "NewEnumerator0"))
  (set `self.ConstructionStatus` ConstructionStatus))

(event `SetBuidingStatus`
  (params (BuildingStatus :type Integer))
  (set `self.BuildingStatus` BuildingStatus)
  (switch `/Game/Core/Enums/Buildings/EConstructuionStatus` (`self.ConstructionStatus`)
    (:`NewEnumerator1`
      _)
    (:`NewEnumerator2`
      _))
  (`self.SetMesh` (`self.BuildingStatus`)))

(event `RunSetPreviewMesh`
  (`self.SetPreviewMesh`)
  (`self.SetPreviewMaterial`))

(fn `AddConstructedTime`
  (params (DeltaConstructionTime :type "Float (double-precision)"))
  (set `self.ConstructionTime` (+ DeltaConstructionTime (`self.ConstructionTime`)))
  (return))

(fn `CalculateSlope`
  (returns (bLocationIsBad :type Boolean))
  (bind _actorlocation (`self.GetVectors`))
  (bind _actorlocation_2 (`self.GetVectors`))
  (bind (_actorlocation_3 _forwardvector _rightvector) (`self.GetVectors`))
  (bind (_actorlocation_4 _forwardvector_2 _rightvector_2) (`self.GetVectors`))
  (bind (_actorlocation_5 _forwardvector_3 _rightvector_3) (`self.GetVectors`))
  (bind (_actorlocation_6 _forwardvector_4 _rightvector_4) (`self.GetVectors`))
  (bind _differences (`self.Differences`))
  (bind (_extent_x _extent_y) (`KismetMathLibrary.BreakVector` (`self.Extent`)))
  (bind _maxdifferenceallowance (`self.MaxdifferenceAllowance`))
  (bind (_indexofminvalue _minvalue) (`KismetMathLibrary.MinOfFloatArray` _differences))
  (bind (_indexofmaxvalue _maxvalue) (`KismetMathLibrary.MaxOfFloatArray` _differences))
  (`KismetArrayLibrary.Array_Clear` (`self.Differences`))
  (`|ExecutionSequence`
    (:`then_0`
      (`|ExecutionSequence`
        (:`then_0`
          (`KismetArrayLibrary.Array_Add` (`self.Differences`) (`self.SlopeTrace` (+ _actorlocation_3 (* (+ _forwardvector _rightvector) (`self.Extent`))))))
        (:`then_1`
          (`KismetArrayLibrary.Array_Add` (`self.Differences`) (`self.SlopeTrace` (+ _actorlocation_4 (* (+ (* _forwardvector_2 -1.0) _rightvector_2) (`self.Extent`))))))
        (:`then_2`
          (`KismetArrayLibrary.Array_Add` (`self.Differences`) (`self.SlopeTrace` (+ _actorlocation_5 (* (+ _forwardvector_3 (* _rightvector_3 -1.0)) (`self.Extent`))))))
        (:`then_3`
          (`KismetArrayLibrary.Array_Add` (`self.Differences`) (`self.SlopeTrace` (+ _actorlocation_6 (* (+ (* _forwardvector_4 -1.0) (* _rightvector_4 -1.0)) (`self.Extent`))))))
        (:`then_4`
          (`KismetArrayLibrary.Array_Add` (`self.Differences`) (`self.SlopeTrace` (`self.GetVectors`))))))
    (:`then_1`
      (if (and (> _indexofminvalue -1) (> _indexofmaxvalue -1))
        (bind (_outhit _returnvalue) (`KismetSystemLibrary.BoxTraceSingle` (+ _actorlocation (0.0 0.0 1000.0)) (- _actorlocation (0.0 0.0 1000.0)) (`KismetMathLibrary.MakeVector` _extent_x _extent_y 1.0) (struct) "TraceTypeQuery1"))
        (if _returnvalue
          (`self.K2_SetActorLocation` (`KismetMathLibrary.MakeVector` (.x _actorlocation_2) (.y _actorlocation_2) (.z (`.ImpactPoint` (`GameplayStatics.BreakHitResult` _outhit))))))))
    (:`then_2`
      (bind _output_get (set `self.bIsOnSlope` (or (> (`KismetMathLibrary.Abs` _minvalue) _maxdifferenceallowance) (> (`KismetMathLibrary.Abs` _maxvalue) _maxdifferenceallowance))))
      (return _output_get))))

(fn `CheckIsOverlapping`
  (returns (bIsOverlapping :type Boolean))
  (return (> (`KismetArrayLibrary.Array_Length` (`self.GetOverlappingActors` null)) 0)))

(fn `DestroyPreview`
  (`StaticMeshComponent.SetStaticMesh` (`self.CurrentBuildingMash`) null)
  (`self.SetEntrance`)
  (`self.SetCollisionArea`)
  (`self.K2_SetActorRotation` (struct))
  (`self.K2_DestroyActor`))

(fn `GetBuidingData`
  (returns (BuildingData :type "/Game/Core/Structures/FBuildingStructure Structure"))
  (return (`self.BuildingData`)))

(fn `GetBuildingRowName`
  (returns (RowName :type Name))
  (return (`self.RowName`)))

(fn `GetBuildingStatus`
  (returns (BuildingStatus :type Integer))
  (return (`self.BuildingStatus`)))

(fn `GetConstructionStatus`
  (returns (ConstructionStatus :type "/Game/Core/Enums/Buildings/EConstructuionStatus Enum"))
  (return (`self.ConstructionStatus`)))

(fn `GetIsOnSlope`
  (returns (bIsOnSlope :type Boolean))
  (return (`self.bIsOnSlope`)))

(fn `GetTimeConstruction`
  (returns (ConstructionTime :type "Float (double-precision)"))
  (return (`self.ConstructionTime`)))

(fn `GetTimeForConstruction`
  (returns (ConstructionTimeToFinish :type "Float (double-precision)"))
  (return (`.ConstructionTime_26_3ADC1B45453F3ADF7CB2B89916F3C368` (break `/Game/Core/Structures/FBuildingStructure` (`self.BuildingData`)))))

(fn `GetVectors`
  (returns (ActorLocation :type "Vector Structure") (ForwardVector :type "Vector Structure") (RightVector :type "Vector Structure"))
  (bind _returnvalue (`self.K2_GetActorRotation`))
  (return (`self.K2_GetActorLocation`) (`KismetMathLibrary.GetRightVector` _returnvalue) (`KismetMathLibrary.GetForwardVector` _returnvalue)))

(fn `MovePreview`
  (params (NewLocation :type "Vector Structure"))
  (`SceneComponent.K2_SetWorldLocation` (`self.CurrentBuildingMash`) NewLocation true true)
  (`self.K2_SetActorLocation` NewLocation true true)
  (`self.SetMaterialOverlap`))

(fn `RotatePreview`
  (params (NewRotation :type "Rotator Structure"))
  (`self.K2_SetActorRotation` NewRotation)
  (return))

(fn `SetBuildingData`
  (returns (DataValid :type Boolean))
  (if (!= (`self.RowName`) "NULL")
    (`self.BuildingDT`
      (:`then`
        (bind _returnvalue (`|GetDataTableRow` "/Game/Core/DataTables/DT_Buildings.DT_Buildings" (`self.RowName`))
          (:`then`
            (set `self.BuildingData` _returnvalue)
            (return true))
          (:`RowNotFound`
            _)))
      (:`else`
        _)))
  (`self.K2_DestroyActor`)
  (return false))

(fn `SetCollisionArea`
  (bind _collisionbox (`self.CollisionBox`))
  (bind (_min _max) (`StaticMeshComponent.GetLocalBounds` (`self.CurrentBuildingMash`)))
  (bind _returnvalue (/ (.z _max) 2.0))
  (`BoxComponent.SetBoxExtent` _collisionbox (`KismetMathLibrary.MakeVector` (- (`KismetMathLibrary.Abs` (.x _min)) 15.0) (- (`KismetMathLibrary.Abs` (.y _min)) 15.0) _returnvalue) true)
  (`SceneComponent.K2_SetRelativeLocation` _collisionbox (`KismetMathLibrary.MakeVector` 0.0 0.0 _returnvalue) false false))

(fn `SetEntrance`
  (bind _entrypoint (`self.EntryPoint`))
  (bind _min (`StaticMeshComponent.GetLocalBounds` (`self.CurrentBuildingMash`)))
  (`BoxComponent.SetBoxExtent` _entrypoint (`KismetMathLibrary.MakeVector` 0.0 (- (`KismetMathLibrary.Abs` (.y _min)) 20.0)) true)
  (`SceneComponent.K2_SetRelativeLocation` _entrypoint (`KismetMathLibrary.MakeVector` (* (+ (`KismetMathLibrary.Abs` (.x _min)) 150.0) -1.0)) false false))

(fn `SetMaterialOverlap`
  (bind _materiallist (`self.MaterialList`))
  (bind _materiallist_2 (`self.MaterialList`))
  (if (or (`self.CheckIsOverlapping`) (`self.CalculateSlope`))
    (for _index (range (`KismetArrayLibrary.Array_Length` _materiallist_2))
      (`MaterialInstanceDynamic.SetVectorParameterValue` (`|GetArrayItem` _materiallist_2 _index) "Color" (struct :`R` 0.520833 :`A` 0.4)))
    (elif (not (and (`self.CheckIsOverlapping`) (`self.CalculateSlope`)))
      (for _index_2 (range (`KismetArrayLibrary.Array_Length` _materiallist))
        (`MaterialInstanceDynamic.SetVectorParameterValue` (`|GetArrayItem` _materiallist _index_2) "Color" (struct :`R` 0.130349 :`G` 1.0 :`B` 0.19211 :`A` 1.0))))))

(fn `SetMesh`
  (params (Indx :type Integer))
  (locals (IndxLocal :type Integer))
  (bind _indxlocal (`local.IndxLocal`))
  (bind (_buildingtype _buildingname _buildinghealth _blsspine _constructionmashes _basicmashes _damagemashes) (break `/Game/Core/Structures/FBuildingStructure` (`self.BuildingData`)))
  (bind _output (`|GetArrayItem` _basicmashes _indxlocal))
  (set `local.IndxLocal` Indx)
  (bind _datavalid (`self.SetBuildingData`))
  (if _datavalid
    (`StaticMeshComponent.SetStaticMesh` (`self.CurrentBuildingMash`) (select `/Game/Core/Enums/Buildings/EConstructuionStatus` (`self.ConstructionStatus`) :`NewEnumerator0` _output :`NewEnumerator1` (`|GetArrayItem` _constructionmashes _indxlocal) :`NewEnumerator2` _output :`NewEnumerator3` (`|GetArrayItem` _damagemashes _indxlocal)))
    (`self.SetCollisionArea`)
    (`self.SetEntrance`)
    (set `self.Extent` (+ (`BoxComponent.GetScaledBoxExtent` (`self.CollisionBox`)) (`BoxComponent.GetScaledBoxExtent` (`self.EntryPoint`))))
    (return)))

(fn `SetPreviewMaterial`
  (bind _currentbuildingmash (`self.CurrentBuildingMash`))
  (bind _previewmaterial (`self.PreviewMaterial`)
    (:`then`
      (for _index (range (+ (`PrimitiveComponent.GetNumMaterials` _currentbuildingmash) 1))
        (`PrimitiveComponent.SetMaterial` _currentbuildingmash _index _previewmaterial)
        (bind _returnvalue (`PrimitiveComponent.CreateDynamicMaterialInstance` _currentbuildingmash _index _previewmaterial "None"))
        (`KismetArrayLibrary.Array_AddUnique` (`self.MaterialList`) _returnvalue)))
    (:`else`)))

(fn `SetPreviewMesh`
  (`self.SetConstructionStatus` "NewEnumerator0")
  (`self.SetMesh` 0))

(fn `SlopeTrace`
  (params (TraceLocation :type "Vector Structure"))
  (returns (Difference :type "Float (double-precision)"))
  (bind (_returnvalue_x _returnvalue_y _returnvalue_z) (`KismetMathLibrary.BreakVector` (`self.K2_GetActorLocation`)))
  (bind _outhit (`KismetSystemLibrary.LineTraceSingle` (+ TraceLocation (0.0 0.0 1000.0)) (- TraceLocation (0.0 0.0 1000.0)) "TraceTypeQuery3"))
  (return (- _returnvalue_z (.z (`.ImpactPoint` (`GameplayStatics.BreakHitResult` _outhit))))))

(fn `UserConstructionScript`
  (`self.SetMesh` 0))
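; Building manager that handles placement previews and timed construction of BP_BuildingMaster actors.
; A looping timer drives the preview, which follows a grid-snapped mouse position, can rotate and reports overlap and slope checks.
; Placement spawns a construction from the stored transform and row name.
; A shared timer, active only while sites exist, advances build time, switches mesh stages by progress (up to four) and moves finished buildings to the completed list.
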(event `SetPreview`
  (params (RowName :type Name))
  (if (`self.bIsPreviewing`)
    (`self.DestroyPreview`))
  (`self.SpawnPreview` RowName)
  (set `self.bIsPreviewing` true)
  (bind _returnvalue (`KismetSystemLibrary.K2_SetTimerDelegate` (`|CreateDelegate` :!event `TrackMouse`) 0.01 true))
  (set `self.PreviewTimerHandle` _returnvalue))

(event `SpawnPreview`
  (params (RowName :type Name))
  (set `self.PreviewTransform` (`KismetMathLibrary.Conv_VectorToTransform` (`self.GetGridSnaps`)))
  (bind _returnvalue (`|SpawnActorFromClass` "/Game/Core/Buildings/BP_BuildingMaster.BP_BuildingMaster_C" (`self.PreviewTransform`) "AdjustIfPossibleButAlwaysSpawn" "MultiplyWithRoot" null RowName "NewEnumerator0" null))
  (`/Engine/EditorBlueprintResources/StandardMacros.IsValid` _returnvalue
    (:`Is Valid`
      (bind _output_get (set `self.BuildingReference` _returnvalue))
      (`/Game/Core/Buildings/BP_BuildingMaster.SetConstructionStatus` _output_get "NewEnumerator0"))))

(event `TrackMouse`
  (bind _buildingreference (`self.BuildingReference`))
  (`/Engine/EditorBlueprintResources/StandardMacros.IsValid` _buildingreference
    (:`Is Valid`
      (`/Game/Core/Buildings/BP_BuildingMaster.MovePreview` _buildingreference (`self.GetGridSnaps`)))))

(event `RotatePreviewLeft`
  (bind _buildingreference (`self.BuildingReference`))
  (bind (_returnvalue_roll _returnvalue_pitch _returnvalue_yaw) (`KismetMathLibrary.BreakRotator` (`Actor.K2_GetActorRotation` _buildingreference)))
  (`/Engine/EditorBlueprintResources/StandardMacros.IsValid` _buildingreference
    (:`Is Valid`
      (`/Game/Core/Buildings/BP_BuildingMaster.RotatePreview` _buildingreference (`KismetMathLibrary.MakeRotator` _returnvalue_roll _returnvalue_pitch (+ _returnvalue_yaw 10.0))))))

(event `RotatePreviewRight`
  (bind _buildingreference (`self.BuildingReference`))
  (bind (_returnvalue_roll _returnvalue_pitch _returnvalue_yaw) (`KismetMathLibrary.BreakRotator` (`Actor.K2_GetActorRotation` _buildingreference)))
  (`/Engine/EditorBlueprintResources/StandardMacros.IsValid` _buildingreference
    (:`Is Valid`
      (`/Game/Core/Buildings/BP_BuildingMaster.RotatePreview` _buildingreference (`KismetMathLibrary.MakeRotator` _returnvalue_roll _returnvalue_pitch (- _returnvalue_yaw 10.0))))))

(event `DestroyPreview`
  (bind _buildingreference (`self.BuildingReference`)
    (:`then`
      (`/Game/Core/Buildings/BP_BuildingMaster.DestroyPreview` _buildingreference)
      (set `self.bIsPreviewing` false)
      (`KismetSystemLibrary.K2_ClearAndInvalidateTimerHandle` (`self.PreviewTimerHandle`)))
    (:`else`)))

(fn `AddToListOfBuildings`
  (params (NewBuilding :type "/Game/Core/Buildings/BP_BuildingMaster Object Reference"))
  (`/Engine/EditorBlueprintResources/StandardMacros.IsValid` NewBuilding
    (:`Is Valid`
      (`KismetArrayLibrary.Array_AddUnique` (`self.ListOfBuildings`) NewBuilding))))

(fn `AddToUnconstructedList`
  (params (NewBuilding :type "/Game/Core/Buildings/BP_BuildingMaster Object Reference"))
  (`/Engine/EditorBlueprintResources/StandardMacros.IsValid` NewBuilding
    (:`Is Valid`
      (`KismetArrayLibrary.Array_AddUnique` (`self.ListOfUnderconstruction`) NewBuilding))))

(fn `GetGridSnaps`
  (returns (GridSnaps :type "Vector Structure"))
  (bind (_mouseposition_x _mouseposition_y _mouseposition_z) (`KismetMathLibrary.BreakVector` (`self.MousePosition`)))
  (bind _snapvalues (`self.SnapValues`))
  (bind _snapvalues_2 (`self.SnapValues`))
  (return (`KismetMathLibrary.MakeVector` (`KismetMathLibrary.Conv_IntToDouble` (* (/ (`KismetMathLibrary.FFloor` (+ _mouseposition_x 50.0)) _snapvalues_2) _snapvalues_2)) (`KismetMathLibrary.Conv_IntToDouble` (* (/ (`KismetMathLibrary.FFloor` (+ _mouseposition_y 50.0)) _snapvalues) _snapvalues)) _mouseposition_z)))

(fn `GetIsPreviewing`
  (returns (bIsPreviewing :type Boolean))
  (return (`self.bIsPreviewing`)))

(fn `GetIsPreviewOnSlope`
  (returns (bIsOnSlope :type Boolean))
  (return (`/Game/Core/Buildings/BP_BuildingMaster.GetIsOnSlope` (`self.BuildingReference`))))

(fn `GetIsPreviewOverlapping`
  (returns (bIsOverlapping :type Boolean))
  (return (`/Game/Core/Buildings/BP_BuildingMaster.CheckIsOverlapping` (`self.BuildingReference`))))

(fn `GetIsPreviewValid`
  (returns (ValidPreview :type Boolean))
  (bind _buildingreference (`self.BuildingReference`))
  (return (and (`KismetSystemLibrary.IsValid` _buildingreference) (`|EnumEquality` (`/Game/Core/Buildings/BP_BuildingMaster.GetConstructionStatus` _buildingreference) "NewEnumerator0"))))

(fn `RemoveFromUnconstructedList`
  (params (OldBuilding :type "/Game/Core/Buildings/BP_BuildingMaster Object Reference"))
  (bind _listofunderconstruction (`self.ListOfUnderconstruction`))
  (`/Engine/EditorBlueprintResources/StandardMacros.IsValid` OldBuilding
    (:`Is Valid`
      (if (>= (`KismetArrayLibrary.Array_Length` _listofunderconstruction) 1)
        (`KismetArrayLibrary.Array_RemoveItem` _listofunderconstruction OldBuilding)))))

(fn `RunConstructionEvent`
  (locals (BuildingLocal :type "/Game/Core/Buildings/BP_BuildingMaster Object Reference") (BuildingToRemoveLocal :type "Array of /Game/Core/Buildings/BP_BuildingMaster Object Reference") (RemovableBuildingLocal :type "/Game/Core/Buildings/BP_BuildingMaster Object Reference"))
  (bind _buildinglocal (`local.BuildingLocal`))
  (bind _buildinglocal_2 (`local.BuildingLocal`))
  (bind _buildinglocal_3 (`local.BuildingLocal`))
  (bind _buildinglocal_4 (`local.BuildingLocal`))
  (bind _buildinglocal_5 (`local.BuildingLocal`))
  (bind _buildinglocal_6 (`local.BuildingLocal`))
  (bind _buildinglocal_7 (`local.BuildingLocal`))
  (bind _buildinglocal_8 (`local.BuildingLocal`))
  (bind _returnvalue (/ (`/Game/Core/Buildings/BP_BuildingMaster.GetTimeConstruction` _buildinglocal_2) (`/Game/Core/Buildings/BP_BuildingMaster.GetTimeForConstruction` _buildinglocal_2)))
  (bind _returnvalue_2 (/ (`/Game/Core/Buildings/BP_BuildingMaster.GetTimeConstruction` _buildinglocal_7) (`/Game/Core/Buildings/BP_BuildingMaster.GetTimeForConstruction` _buildinglocal_7)))
  (bind _returnvalue_3 (/ (`/Game/Core/Buildings/BP_BuildingMaster.GetTimeConstruction` _buildinglocal_8) (`/Game/Core/Buildings/BP_BuildingMaster.GetTimeForConstruction` _buildinglocal_8)))
  (if (>= (`KismetArrayLibrary.Array_Length` (`self.ListOfUnderconstruction`)) 1)
    (for _array_element (`self.ListOfUnderconstruction`)
      (set `local.BuildingLocal` _array_element)
      (if (`|EnumEquality` (`/Game/Core/Buildings/BP_BuildingMaster.GetConstructionStatus` (`local.BuildingLocal`)) "NewEnumerator1")
        (`/Game/Core/Buildings/BP_BuildingMaster.AddConstructedTime` (`local.BuildingLocal`) (`self.BaseConstructionSpeed`))
        (switch `int` (`KismetArrayLibrary.Array_Length` (`.ConstructionMashes_36_C24424D4436AD4304B735E8E64F4968F` (break `/Game/Core/Structures/FBuildingStructure` (`/Game/Core/Buildings/BP_BuildingMaster.GetBuidingData` (`local.BuildingLocal`)))))
          (:`1`
            _)
          (:`2`
            ;[1 1 1] Meshes Update System. If more - need more branches
            (if (and (>= (/ (`/Game/Core/Buildings/BP_BuildingMaster.GetTimeConstruction` _buildinglocal_5) (`/Game/Core/Buildings/BP_BuildingMaster.GetTimeForConstruction` _buildinglocal_5)) 0.55) (!= (`/Game/Core/Buildings/BP_BuildingMaster.GetBuildingStatus` _buildinglocal_5) 1))
              (`/Game/Core/Buildings/BP_BuildingMaster.SetBuidingStatus` (`local.BuildingLocal`) 1)))
          (:`3`
            (if (and (and (>= _returnvalue_3 0.33) (< _returnvalue_3 0.66)) (!= (`/Game/Core/Buildings/BP_BuildingMaster.GetBuildingStatus` _buildinglocal_8) 1))
              (`/Game/Core/Buildings/BP_BuildingMaster.SetBuidingStatus` (`local.BuildingLocal`) 1))
            (if (and (>= (/ (`/Game/Core/Buildings/BP_BuildingMaster.GetTimeConstruction` _buildinglocal_4) (`/Game/Core/Buildings/BP_BuildingMaster.GetTimeForConstruction` _buildinglocal_4)) 0.66) (!= (`/Game/Core/Buildings/BP_BuildingMaster.GetBuildingStatus` _buildinglocal_4) 2))
              (`/Game/Core/Buildings/BP_BuildingMaster.SetBuidingStatus` (`local.BuildingLocal`) 2)))
          (:`4`
            (if (and (and (>= _returnvalue_2 0.25) (< _returnvalue_2 0.5)) (!= (`/Game/Core/Buildings/BP_BuildingMaster.GetBuildingStatus` _buildinglocal_7) 1))
              (`/Game/Core/Buildings/BP_BuildingMaster.SetBuidingStatus` (`local.BuildingLocal`) 1))
            (if (and (and (>= _returnvalue 0.5) (< _returnvalue 0.75)) (!= (`/Game/Core/Buildings/BP_BuildingMaster.GetBuildingStatus` _buildinglocal_2) 2))
              (`/Game/Core/Buildings/BP_BuildingMaster.SetBuidingStatus` (`local.BuildingLocal`) 2))
            (if (and (>= (/ (`/Game/Core/Buildings/BP_BuildingMaster.GetTimeConstruction` _buildinglocal_3) (`/Game/Core/Buildings/BP_BuildingMaster.GetTimeForConstruction` _buildinglocal_3)) 0.75) (!= (`/Game/Core/Buildings/BP_BuildingMaster.GetBuildingStatus` _buildinglocal_3) 3))
              (`/Game/Core/Buildings/BP_BuildingMaster.SetBuidingStatus` (`local.BuildingLocal`) 3))))
        (if (>= (`/Game/Core/Buildings/BP_BuildingMaster.GetTimeConstruction` _buildinglocal_6) (`/Game/Core/Buildings/BP_BuildingMaster.GetTimeForConstruction` _buildinglocal_6))
          (`KismetArrayLibrary.Array_Add` (`local.BuildingToRemoveLocal`) (`local.BuildingLocal`))
          (`/Game/Core/Buildings/BP_BuildingMaster.SetConstructionStatus` _buildinglocal "NewEnumerator2")
          (`/Game/Core/Buildings/BP_BuildingMaster.SetBuidingStatus` _buildinglocal 0))))
    (for _array_element_2 (`local.BuildingToRemoveLocal`)
      (bind _output_get (set `local.RemovableBuildingLocal` _array_element_2))
      (`self.RemoveFromUnconstructedList` _output_get)
      (`self.AddToListOfBuildings` _output_get))
    (`KismetArrayLibrary.Array_Clear` (`local.BuildingToRemoveLocal`))
    (if (<= (`KismetArrayLibrary.Array_Length` (`self.ListOfUnderconstruction`)) 0)
      (`KismetSystemLibrary.K2_ClearAndInvalidateTimerHandle` (`self.ConstructionTimerHandle`)))
    (elif (<= (`KismetArrayLibrary.Array_Length` (`self.ListOfUnderconstruction`)) 0)
      (`KismetSystemLibrary.K2_ClearAndInvalidateTimerHandle` (`self.ConstructionTimerHandle`)))))

(fn `SetConstructionTimer`
  (bind _constructiontimerhandle (`self.ConstructionTimerHandle`))
  (if (>= (`KismetArrayLibrary.Array_LastIndex` (`self.ListOfUnderconstruction`)) 0)
    (if (not (`KismetSystemLibrary.K2_IsTimerActiveHandle` (`self.ConstructionTimerHandle`)))
      (bind _returnvalue (`KismetSystemLibrary.K2_SetTimer` null "RunConstructionEvent" (`self.BaseConstructionSpeed`) true))
      (set `self.ConstructionTimerHandle` _returnvalue))
    (elif (or (`KismetSystemLibrary.K2_IsTimerActiveHandle` _constructiontimerhandle) (`KismetSystemLibrary.K2_IsValidTimerHandle` _constructiontimerhandle))
      (`KismetSystemLibrary.K2_ClearAndInvalidateTimerHandle` (`self.ConstructionTimerHandle`)))))

(fn `SetIsPreviewing`
  (params (bIsPreviewing :type Boolean))
  (set `self.bIsPreviewing` bIsPreviewing)
  (return))

(fn `SetMousePosition`
  (params (MousePosition :type "Vector Structure"))
  (set `self.MousePosition` MousePosition)
  (return))

(fn `SpawnConstruction`
  (locals (BuildingLocal :type "/Game/Core/Buildings/BP_BuildingMaster Object Reference"))
  (bind _returnvalue (`|SpawnActorFromClass` "/Game/Core/Buildings/BP_BuildingMaster.BP_BuildingMaster_C" (`self.BuildingTransform`) "Undefined" "MultiplyWithRoot" null (`self.BuildingRowName`) "NewEnumerator1" null))
  (if (!= _returnvalue null)
    (bind _output_get (set `local.BuildingLocal` _returnvalue))
    (`/Game/Core/Buildings/BP_BuildingMaster.SetBuidingStatus` _output_get 0)
    (`self.AddToUnconstructedList` _output_get)
    (`self.SetConstructionTimer`)))

(fn `StoreVariables`
  (bind _buildingreference (`self.BuildingReference`))
  (set `self.BuildingTransform` (`Actor.GetTransform` _buildingreference))
  (set `self.BuildingRowName` (`/Game/Core/Buildings/BP_BuildingMaster.GetBuildingRowName` _buildingreference))
  (return))